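; BP_MainGameMode is the game mode that handles player spawning, death stats and post-death spectating.
; SpawnPlayer destroys any existing pawn, picks a random available BP_GameStartPosition matching the player's tag, and has it spawn the character.
; CharacterDead records kill and death on the player states, notifies the victim's state, then has the victim's controller possess a BP_GameSpectorToChar that follows the killer.
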(event EventPostLogin
  (params (NewPlayer :type Player%20Controller%20Object%20Reference)))

(fn ConstructionScript)

(fn CharacterDead
  (params (DeadCharacter :type BP%20Main%20Character%20Object%20Reference) (DeathInstigator :type BP%20Main%20Controler%20Object%20Reference) (DeathFrom :type Actor%20Object%20Reference))
  ;[1 1 1] Update stat info and posses controler to spector pawn when character is dead
  (LocalVariables|SetL_Character DeadCharacter)
  (LocalVariables|SetL_Instigator DeathInstigator)
  (LocalVariables|SetL_DeadFrom DeathFrom)
  (Utilities|FlowControl|Sequence
    (:then_0
      (CallFunction|UpdateDeathInfo (LocalVariables|GetL_Instigator) (LocalVariables|GetL_Character)))
    (:then_1
      (Default|OwnedCharacterDead (.AsBP%20Main%20Player%20State (Utilities|Casting|CastToBP_MainPlayerState (Variables|/Script/Engine.Pawn|GetPlayerState (LocalVariables|GetL_Character)))) (.AsBP%20Main%20Character (Utilities|Casting|CastToBP_MainCharacter (Pawn|GetControlledPawn (LocalVariables|GetL_Instigator))))))
    (:then_2
      (CallFunction|SpawninSpector (.AsBP%20Main%20Controler (Utilities|Casting|CastToBP_MainControler (Pawn|GetController (LocalVariables|GetL_Character)))) (LocalVariables|GetL_Instigator)))))

(fn SpawnPlayer
  (params (PlayerControler :type BP%20Main%20Controler%20Object%20Reference))
  (bind _returnvalue (Pawn|GetControlledPawn PlayerControler))
  ;[1 1 1] Spawn player in available start position
  (Utilities|IsValid _returnvalue
    (:Is%20Valid
      (Actor|DestroyActor _returnvalue))
    (:Is%20Not%20Valid
      _))
  (bind _availablepoint (CallFunction|FindAvailablePoint PlayerControler))
  (bind _output_get (LocalVariables|SetL_PlayerPosition (Utilities|Array|Get(acopy) _availablepoint (Math|Random|RandomInteger (Utilities|Array|LastIndex _availablepoint)))))
  (Default|SpawnCharacter _output_get PlayerControler)
  (Variables|/Game/OMPST_V2/Blueprints/State/BP_MainPlayerState.BP_MainPlayerState_C|SetCharacterAlive (.AsBP%20Main%20Player%20State (Utilities|Casting|CastToBP_MainPlayerState (Variables|/Script/Engine.Controller|GetPlayerState PlayerControler))) true))

(fn FindAvailablePoint
  (params (PlayerControler :type BP%20Main%20Controler%20Object%20Reference))
  ;[1 1 1] Looking for available start position
  (bind _outactors (Actor|GetAllActorsOfClass "/Game/OMPST_V2/Blueprints/LevelComponent/BP_GameStartPosition.BP_GameStartPosition_C"))
  (for _array_element _outactors
    (if (and (Default|AvailablePoint _array_element) (Utilities|Name|Equal(Name) (Variables|/Script/Engine.PlayerStart|GetPlayerStartTag _array_element) (Variables|/Game/OMPST_V2/Blueprints/State/BP_MainPlayerState.BP_MainPlayerState_C|GetPlayerTag (.AsBP%20Main%20Player%20State (Utilities|Casting|CastToBP_MainPlayerState (Variables|/Script/Engine.Controller|GetPlayerState PlayerControler))))))
      (Utilities|Array|Add (LocalVariables|GetL_AvailablePoint) _array_element)))
  (return (LocalVariables|GetL_AvailablePoint)))

(fn SpawninSpector
  (params (DeadController :type BP%20Main%20Controler%20Object%20Reference) (DeathInstigator :type BP%20Main%20Controler%20Object%20Reference))
  ;[1 1 1] Send player controller  to death instigator to follow
  (LocalVariables|SetL_DeadControler DeadController)
  (bind _output_get (LocalVariables|SetL_DeathInstigator DeathInstigator))
  (Utilities|IsValid _output_get
    (:Is%20Valid
      (bind _returnvalue (Game|SpawnActorfromClass "/Game/OMPST_V2/Blueprints/Player/BP_GameSpectorToChar.BP_GameSpectorToChar_C" (Transformation|GetActorTransform (Pawn|GetControlledPawn (LocalVariables|GetL_DeadControler))) "Undefined" (LocalVariables|GetL_DeadControler) 0 0))
      (LocalVariables|SetL_Spector _returnvalue)
      (Pawn|Possess (LocalVariables|GetL_DeadControler) (LocalVariables|GetL_Spector))
      (bind _asbp_game_spector_to_char (Utilities|Casting|CastToBP_GameSpectorToChar (LocalVariables|GetL_Spector))
        (:then
          (Default|AddCharactertoFollow _asbp_game_spector_to_char (.AsBP%20Main%20Character (Utilities|Casting|CastToBP_MainCharacter (Pawn|GetControlledPawn (LocalVariables|GetL_DeathInstigator))))))
        (:CastFailed
          _))
      (return (LocalVariables|GetL_Spector)))))

(fn UpdateDeathInfo
  (params (Instigator :type BP%20Main%20Controler%20Object%20Reference) (Character :type BP%20Main%20Character%20Object%20Reference))
  ;[1 1 1] Update info
  (Default|AddKill (.AsBP%20Main%20Player%20State (Utilities|Casting|CastToBP_MainPlayerState (Variables|/Script/Engine.Controller|GetPlayerState Instigator))))
  (Default|AddDeath (.AsBP%20Main%20Player%20State (Utilities|Casting|CastToBP_MainPlayerState (Variables|/Script/Engine.Controller|GetPlayerState (Pawn|GetController Character))))))