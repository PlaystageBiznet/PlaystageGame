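; BP_MainGameState is the match game state that detects when the kill limit is reached in team or free-for-all play.
; Shortly after BeginPlay, the server copies the limit and mode from BP_OnlineInstance, then starts a looping timer that polls either Alpha/Delta team totals or each player state's kills.
; A hit sets KillLimitDone, plus the winning team name in team mode.
; It also relays new player connections through a dispatcher.
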(event Custom|KillLimitEnd
  ;[1 1 1] Set kill limit, and check it every 0.1sec
  (bind _array_element (Utilities|Array|ForEachLoopwithBreak (Variables|Default|GetPlayerArray) :!label _label)
    (:LoopBody
      (bind _asbp_main_player_state (Utilities|Casting|CastToBP_MainPlayerState _array_element))
      (if (== (Variables|/Game/OMPST_V2/Blueprints/State/BP_MainPlayerState.BP_MainPlayerState_C|GetKills _asbp_main_player_state) (Variables|Default|GetKillLimit))
        (Variables|Default|SetKillLimitDone true)
        (goto _label Break)))))

(event Custom|TeamKillLimitCheck
  ;[1 1 1] Set kill limit, and check it every 0.1sec
  (if (>= (Variables|Default|GetAlphaTeamKill) (Variables|Default|GetKillLimit))
    (Variables|Default|SetKillLimitDone true)
    (Variables|Default|SetMaxTeamKiller "Alpha")
    (elif (>= (Variables|Default|GetDeltaTeamKill) (Variables|Default|GetKillLimit))
      (Variables|Default|SetKillLimitDone true)
      (Variables|Default|SetMaxTeamKiller "Delta"))))

(event EventBeginPlay
  ;[1 1 1] Set kill limit, and check it every 0.1sec
  (Utilities|FlowControl|Delay 0.2)
  (Networking|SwitchHasAuthority
    (:Authority
      (Variables|Default|SetKillLimit (Variables|/Game/OMPST_V2/Blueprints/Instance/BP_OnlineInstance.BP_OnlineInstance_C|GetKillLimitPasser (.AsBP%20Online%20Instance (Utilities|Casting|CastToBP_OnlineInstance (Game|GetGameInstance)))))
      (Variables|Default|SetisTeamMatch (Variables|/Game/OMPST_V2/Blueprints/Instance/BP_OnlineInstance.BP_OnlineInstance_C|GetisTeamMatch (.AsBP%20Online%20Instance (Utilities|Casting|CastToBP_OnlineInstance (Game|GetGameInstance)))))
      (if (Variables|Default|GetisTeamMatch)
        (Utilities|Time|SetTimerbyEvent (delegate Custom|TeamKillLimitCheck) 0.1 true)
        (else
          (Utilities|Time|SetTimerbyEvent (delegate Custom|KillLimitEnd) 0.1 true))))))

(fn ConstructionScript)

(fn OnRepRoundinProgress)

(fn NewPlayerConnectedtoServer
  (params (NewPlayerState :type BP%20Main%20Player%20State%20Object%20Reference))
  (Default|CallNewPlayerConnected NewPlayerState))