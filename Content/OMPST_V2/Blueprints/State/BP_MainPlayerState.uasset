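; Multiplayer shooter PlayerState that tracks kills, deaths, money, alive status and the Alpha/Delta team tag.
; Kills and deaths adjust clamped money; kills also feed GameState team scores, and Tick records MaxKiller at the kill limit.
; The CharacterAlive RepNotify, gated to the server, triggers events swapping HUD and solo or team spectator widgets.
; It reports joins to GameState after a delay, relays deaths through CallOwnedCharIsDead, and multicasts the ready tag.
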(event Custom|-addMoney
  ;[1 1 1] Money
  (if (<= (Variables|Default|GetMoney) 949)
    (Variables|Default|SetMoney (+ (Variables|Default|GetMoney) 50))
    (else
      (Variables|Default|SetMoney 999))))

(event Custom|ReadyToPlayServer
  (params (Condition :type Name))
  ;[1 1 1] Set player condition "ready to play"
  (CallFunction|ReadytoPlayMulticast self Condition))

(event Custom|-takeMoney
  ;[1 1 1] Money
  (if (>= (Variables|Default|GetMoney) 25)
    (Variables|Default|SetMoney (- (Variables|Default|GetMoney) 25))
    (else
      (Variables|Default|SetMoney 0))))

(event Custom|ReadyToPlayMulticast
  (params (Condition :type Name))
  ;[1 1 1] Set player condition "ready to play"
  (Variables|Default|SetPlayerTag Condition)
  (CallFunction|SetPlayerReadytoPlay self Condition))

(event Custom|RemoveMainWG
  ;[1 1 1] Add and remove widgets
  (CallFunction|RemoveMainWidget))

(event Custom|AddMainWG
  ;[1 1 1] Add and remove widgets
  (CallFunction|AddMainWidget))

(event Custom|AddDeadSpectatorWG
  ;[1 1 1] Add and remove widgets
  (CallFunction|AddDeadSpectatorWidget))

(event Custom|OwnedCharacterDead
  (params (DeathInstigator :type BP%20Main%20Character%20Object%20Reference))
  ;[1 1 1] Call everywhere that character is dead
  (Default|CallOwnedCharIsDead DeathInstigator self DeathInstigator))

(event EventTick
  (params (DeltaSeconds :type Float%20%28single-precision%29))
  ;[1 1 1] Check round condition
  (bind _asbp_main_game_state (Utilities|Casting|CastToBP_MainGameState (Game|GetGameState)))
  (if (>= (Variables|Default|GetKills) (Variables|/Game/OMPST_V2/Blueprints/State/BP_MainGameState.BP_MainGameState_C|GetKillLimit _asbp_main_game_state))
    (Variables|/Game/OMPST_V2/Blueprints/State/BP_MainGameState.BP_MainGameState_C|SetMaxKiller (.AsBP%20Main%20Game%20State (Utilities|Casting|CastToBP_MainGameState (Game|GetGameState))) (PlayerState|GetPlayerName))))

(event EventBeginPlay
  ;[1 1 1] Call everywhere that new player is connected
  (Utilities|FlowControl|Delay 2.0)
  (Default|NewPlayerConnectedtoServer (.AsBP%20Main%20Game%20State (Utilities|Casting|CastToBP_MainGameState (Game|GetGameState)))))

(fn ConstructionScript)

(fn AddKill
  (bind _returnvalue (Game|GetGameState))
  (bind _asbp_main_game_state (Utilities|Casting|CastToBP_MainGameState _returnvalue))
  (Math|Integer|IncrementInt (Variables|Default|GetKills)
    (:%20%20
      (CallFunction|-addMoney)
      (if (Utilities|Name|Equal(Name) (Variables|Default|GetPlayerTag) "Alpha")
        (Variables|/Game/OMPST_V2/Blueprints/State/BP_MainGameState.BP_MainGameState_C|SetAlphaTeamKill _asbp_main_game_state (+ (Variables|/Game/OMPST_V2/Blueprints/State/BP_MainGameState.BP_MainGameState_C|GetAlphaTeamKill _asbp_main_game_state) 1))
        (else
          (Variables|/Game/OMPST_V2/Blueprints/State/BP_MainGameState.BP_MainGameState_C|SetDeltaTeamKill _asbp_main_game_state (+ (Variables|/Game/OMPST_V2/Blueprints/State/BP_MainGameState.BP_MainGameState_C|GetDeltaTeamKill _asbp_main_game_state) 1)))))))

(fn AddDeath
  (Math|Integer|IncrementInt (Variables|Default|GetDeaths)
    (:%20%20
      (Variables|Default|SetCharacterAlive false)
      (CallFunction|-takeMoney))))

(fn OnRepCharacterAlive
  ;[1 1 1] Add and remove widgets when player is dead or alive
  (if (Variables|Default|GetCharacterAlive)
    (if (Networking|IsServer)
      (CallFunction|AddMainWG))
    (elif (< (Variables|Default|GetKills) (Variables|/Game/OMPST_V2/Blueprints/State/BP_MainGameState.BP_MainGameState_C|GetKillLimit (.AsBP%20Main%20Game%20State (Utilities|Casting|CastToBP_MainGameState (Game|GetGameState)))))
      (if (Networking|IsServer)
        (CallFunction|RemoveMainWG)
        (CallFunction|AddDeadSpectatorWG)))))

(fn SetPlayerReadytoPlay
  (params (Condition :type Name))
  ;[1 1 1] Add to ready to start tag
  (Utilities|Array|Add (Variables|Actor|GetTags) Condition))

(fn RemoveMainWidget
  (bind _returnvalue (Game|GetPlayerController 0))
  ;[1 1 1] Remove Main Widget
  (bind _foundwidgets (Widget|GetAllWidgetsOfClass "/Game/OMPST_V2/Widgets/WG_Main.WG_Main_C" true))
  (Widget|RemovefromParent _foundwidgets)
  (bind _foundwidgets_2 (Widget|GetAllWidgetsOfClass "/Game/OMPST_V2/Widgets/InGame/WG_Shop.WG_Shop_C" true))
  (Widget|RemovefromParent _foundwidgets_2)
  (Input|SetInputModeGameOnly _returnvalue)
  (Variables|/Script/Engine.PlayerController|SetbShowMouseCursor _returnvalue false))

(fn AddMainWidget
  ;[1 1 1] Add Main Widget
  (bind _returnvalue (UserInterface|CreateWidget "/Game/OMPST_V2/Widgets/WG_Main.WG_Main_C" (Game|GetPlayerController 0)))
  (UserInterface|Viewport|AddtoViewport _returnvalue 0))

(fn AddDeadSpectatorWidget
  (bind _returnvalue (Game|GetPlayerController 0))
  ;[1 1 1] Add Dead Spectator Widget
  (if (Variables|/Game/OMPST_V2/Blueprints/State/BP_MainGameState.BP_MainGameState_C|GetisTeamMatch (.AsBP%20Main%20Game%20State (Utilities|Casting|CastToBP_MainGameState (Game|GetGameState))))
    (bind _returnvalue_2 (UserInterface|CreateWidget "/Game/OMPST_V2/Widgets/DeadSpectator/WG_TeamDeadSpectator.WG_TeamDeadSpectator_C" _returnvalue))
    (UserInterface|Viewport|AddtoViewport _returnvalue_2 0)
    (else
      (bind _returnvalue_3 (UserInterface|CreateWidget "/Game/OMPST_V2/Widgets/DeadSpectator/WG_DeadSpectator.WG_DeadSpectator_C" _returnvalue))
      (UserInterface|Viewport|AddtoViewport _returnvalue_3 0))))