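; Game start point that tracks whether a main character occupies it and can spawn a character for a controller.
; Capsule overlap events set and clear CharacterInside, which AvailablePoint checks to report whether the point is free.
; SpawnCharacter spawns PersonCharacter at its own transform, owned by the given controller.
; It then sets CharacterInside to None and uses that variable, not the spawn result, for Possess and the return value.
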(event OnComponentEndOverlap(CapsuleComponent)
  (params (OverlappedComponent :type Primitive%20Component%20Object%20Reference) (OtherActor :type Actor%20Object%20Reference) (OtherComp :type Primitive%20Component%20Object%20Reference) (OtherBodyIndex :type Integer))
  (if (== OtherActor (Variables|Default|GetCharacterInside))
    (Variables|Default|SetCharacterInside 0)))

(event OnComponentBeginOverlap(CapsuleComponent)
  (params (OverlappedComponent :type Primitive%20Component%20Object%20Reference) (OtherActor :type Actor%20Object%20Reference) (OtherComp :type Primitive%20Component%20Object%20Reference) (OtherBodyIndex :type Integer) (bFromSweep :type Boolean) (SweepResult :type Hit%20Result%20Structure%20%28by%20ref%29))
  (bind _asbp_main_character (Utilities|Casting|CastToBP_MainCharacter OtherActor))
  (Variables|Default|SetCharacterInside _asbp_main_character))

(fn ConstructionScript)

(fn AvailablePoint
  (Utilities|IsValid (Variables|Default|GetCharacterInside)
    (:Is%20Valid
      (return false))
    (:Is%20Not%20Valid
      (return true))))

(fn SpawnCharacter
  (params (Controler :type BP%20Main%20Controler%20Object%20Reference))
  (Game|SpawnActorfromClass "/Game/Blueprints/PersonCharacter.PersonCharacter_C" (Transformation|GetActorTransform) "Undefined" Controler 0)
  (bind _output_get (Variables|Default|SetCharacterInside 0))
  (Pawn|Possess Controler _output_get)
  (return _output_get))