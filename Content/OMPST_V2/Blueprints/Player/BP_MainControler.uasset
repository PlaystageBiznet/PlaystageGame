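; Main player controller for a multiplayer shooter, handling chat, respawning and the round-end screen.
; Enter opens the HUD chat widget, and sent messages go to the GameState's chat manager.
; Respawns call the GameMode's SpawnPlayer, either after a timer or through a server-to-multicast event chain.
; Tick polls the GameState's kill limit, then once shows a team or solo end screen, switches to UI-only input and empties weapon ammo.
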(event Custom|RespawnServer
  ;[1 1 1] Respawn Players for start
  (CallFunction|RespawnMulticast))

(event Custom|RespawnEvent
  ;[1 1 1] Respawn Players for start
  (CallFunction|RespawnServer))

(event Custom|RespawnMulticast
  ;[1 1 1] Respawn Players for start
  (CallFunction|Respawn))

(event Custom|SendMessageServer
  (params (Message :type Text))
  ;[1 1 1] Chat
  (Default|SendMessage (Variables|/Game/OMPST_V2/Blueprints/State/BP_MainGameState.BP_MainGameState_C|GetBP_ChatManager (.AsBP%20Main%20Game%20State (Utilities|Casting|CastToBP_MainGameState (Game|GetGameState)))) Message (.AsBP%20Main%20Player%20State (Utilities|Casting|CastToBP_MainPlayerState (Variables|GetPlayerState)))))

(event EventTick
  (params (DeltaSeconds :type Float%20%28single-precision%29))
  (bind _returnvalue (Game|GetPlayerController 0))
  ;[1 1 1] Round end
  (bind _asbp_main_game_state (Utilities|Casting|CastToBP_MainGameState (Game|GetGameState)))
  (if (Variables|/Game/OMPST_V2/Blueprints/State/BP_MainGameState.BP_MainGameState_C|GetKillLimitDone _asbp_main_game_state)
    (Utilities|FlowControl|DoOnce false
      (:Completed
        (Viewport|RemoveAllWidgets)
        (if (Variables|/Game/OMPST_V2/Blueprints/State/BP_MainGameState.BP_MainGameState_C|GetisTeamMatch _asbp_main_game_state)
          (bind _returnvalue_2 (UserInterface|CreateWidget "/Game/OMPST_V2/Widgets/RoundEnd/WG_TeamRoundEnd.WG_TeamRoundEnd_C" _returnvalue))
          (UserInterface|Viewport|AddtoViewport _returnvalue_2 0)
          (else
            (bind _returnvalue_3 (UserInterface|CreateWidget "/Game/OMPST_V2/Widgets/RoundEnd/WG_RoundEnd.WG_RoundEnd_C" _returnvalue))
            (UserInterface|Viewport|AddtoViewport _returnvalue_3 0)))
        (Input|SetInputModeUIOnly _returnvalue 0 "DoNotLock")
        (Variables|/Script/Engine.PlayerController|SetbShowMouseCursor _returnvalue true)
        (Utilities|IsValid 0
          (:Is%20Valid
            (Variables|/Game/OMPST_V2/Weapons/BP_Weapon.BP_Weapon_C|SetAmmoCurrent (Default|ToWeapon (.AsBP%20Main%20Character (Utilities|Casting|CastToBP_MainCharacter (Pawn|GetControlledPawn _returnvalue)))) 0)))))))

(event Input|KeyboardEvents|N
  (params (Key :type Key%20Structure :default "None")))

(event Input|KeyboardEvents|Enter
  (params (Key :type Key%20Structure :default "None"))
  ;[1 1 1] Chat
  (:Pressed
    (Default|ActivateChatWidget (.AsBP%20Main%20Hud (Utilities|Casting|CastToBP_MainHud (HUD|GetHUD (Game|GetPlayerController 0)))) true)))

(event Input|KeyboardEvents|M
  (params (Key :type Key%20Structure :default "None")))

(fn ConstructionScript)

(fn Respawn
  (bind _asbp_main_game_mode (Utilities|Casting|CastToBP_MainGameMode (Game|GetGameMode)))
  (Default|SpawnPlayer _asbp_main_game_mode self))

(fn StartRespawnTimer
  (bind _returnvalue (Utilities|Time|SetTimerbyFunctionName 0 "Respawn" 5.0))
  (Variables|Default|SetRespawnTimer _returnvalue))

(fn -roundEnd)