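; Spectator pawn that a player controls after death, trailing the character passed to it, noted as the death instigator.
; Each tick it smoothly interpolates its location toward that character, with the follow speed set one second after BeginPlay.
; Pressing U or calling RespawnEvent requests a respawn from BP_MainControler, then targets the team or non-team dead-spectator widgets for removal based on the game state's match type.
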(event Custom|RespawnEvent
  ;[1 1 1] Manual Respawn
  (Default|RespawnEvent (.AsBP%20Main%20Controler (Utilities|Casting|CastToBP_MainControler (Pawn|GetController))))
  (if (Variables|/Game/OMPST_V2/Blueprints/State/BP_MainGameState.BP_MainGameState_C|GetisTeamMatch (.AsBP%20Main%20Game%20State (Utilities|Casting|CastToBP_MainGameState (Game|GetGameState))))
    (bind _foundwidgets (Widget|GetAllWidgetsOfClass "/Game/OMPST_V2/Widgets/DeadSpectator/WG_TeamDeadSpectator.WG_TeamDeadSpectator_C" true))
    (Widget|RemovefromParent _foundwidgets)
    (else
      (bind _foundwidgets_2 (Widget|GetAllWidgetsOfClass "/Game/OMPST_V2/Widgets/DeadSpectator/WG_DeadSpectator.WG_DeadSpectator_C" true))
      (Widget|RemovefromParent _foundwidgets_2))))

(event EventBeginPlay
  ;[1 1 1] Set speed and location for your controller when sending your controller to death instigator
  (Utilities|FlowControl|Delay 1.0)
  (Variables|Default|SetSpeed 15.0))

(event EventTick
  (params (DeltaSeconds :type Float%20%28single-precision%29))
  ;[1 1 1] Set speed and location for your controller when sending your controller to death instigator
  (bind _charactertofollow (Variables|Default|GetCharacterToFollow)
    (:then
      (Transformation|SetActorLocation (Math|Interpolation|VInterpTo (Transformation|GetActorLocation) (Transformation|GetActorLocation _charactertofollow) (Utilities|Time|GetWorldDeltaSeconds) (Variables|Default|GetSpeed)) false false))
    (:else)))

(event Input|KeyboardEvents|U
  (params (Key :type Key%20Structure))
  ;[1 1 1] Manual Respawn
  (:Pressed
    (CallFunction|RespawnEvent)))

(fn ConstructionScript
  (|CallParentFunction))

(fn AddCharactertoFollow
  (params (Player :type BP%20Main%20Character%20Object%20Reference))
  (Variables|Default|SetCharacterToFollow Player))