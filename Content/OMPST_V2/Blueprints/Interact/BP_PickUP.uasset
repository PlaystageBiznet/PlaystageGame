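; BP_PickUP is a pickup actor that displays its name through a widget when the player character is nearby.
; Tick casts the player pawn to BP_MainCharacter, caches it, and compares its distance to VisibilityDistance to show or hide the name.
; The WG_PickUp widget is created lazily on first show using InteractST.Name, then only its component's visibility is toggled.
; The Interact event is an empty stub.
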(event Custom|Interact
  (params (Character :type BP%20Main%20Character%20Object%20Reference)))

(event Custom|-ShowName
  (bind _widget (Variables|Default|GetWidget))
  ;[1 1 1] Show/Hide name
  (Utilities|IsValid (Variables|Default|GetWG_Name)
    (:Is%20Valid
      (Rendering|SetVisibility _widget true false))
    (:Is%20Not%20Valid
      (bind _returnvalue (UserInterface|CreateWidget "/Game/OMPST_V2/Widgets/Interact/WG_PickUp.WG_PickUp_C" 0 (Utilities|Struct|BreakBP_S_Interact (Variables|Default|GetInteractST))))
      (bind _output_get (Variables|Default|SetWG_Name _returnvalue))
      (UserInterface|SetWidget _widget _output_get))))

(event Custom|-HideName
  ;[1 1 1] Show/Hide name
  (Rendering|SetVisibility (Variables|Default|GetWidget) false false))

(event EventTick
  (params (DeltaSeconds :type Float%20%28single-precision%29))
  ;[1 1 1] Tick
  (bind _asbp_main_character (Utilities|Casting|CastToBP_MainCharacter (Game|Player|GetPlayerPawn 0)))
  (Variables|Default|SetToCharacter _asbp_main_character)
  (if (< (Math|Vector|Distance(Vector) (Transformation|GetActorLocation _asbp_main_character) (Transformation|GetActorLocation)) (Variables|Default|GetVisibilityDistance))
    (CallFunction|-ShowName)
    (else
      (CallFunction|-HideName))))

(fn ConstructionScript)