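; BP_PickUP_Sniper is an interactable pickup that gives a character the sniper rifle.
; On Interact, if the character's BPWeaponManager has no valid sniper rifle, it attaches one, copies over the pickup's current and total ammo, then destroys itself.
; A separate attachWeapon function, not called in this file, spawns and attaches a hidden shotgun instead, apparently left over from a shotgun pickup.
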(event EventBeginPlay)

(event Collision|EventActorBeginOverlap
  (params (OtherActor :type Actor%20Object%20Reference)))

(event EventTick
  (params (DeltaSeconds :type Float%20%28single-precision%29))
  (|CallParentFunction DeltaSeconds) ; This node is disabled and will not be called.\nDrag off pins to build functionality.
)

(event EventInteract
  (params (Character :type BP%20Main%20Character%20Object%20Reference))
  (bind _bp_weaponmanager (Variables|/Game/OMPST_V2/Blueprints/Player/BP_MainCharacter.BP_MainCharacter_C|GetBP_WeaponManager Character))
  (|CallParentFunction Character)
  (Utilities|IsValid (Variables|/Game/OMPST_V2/Weapons/Data/BP_WeaponManager.BP_WeaponManager_C|GetSniperRifle_Weapon _bp_weaponmanager)
    (:Is%20Not%20Valid
      (bind _attachedweapon (Default|AttachWeapon _bp_weaponmanager "/Game/OMPST_V2/Weapons/BP_Weapon_SniperRifle.BP_Weapon_SniperRifle_C"))
      (Variables|/Game/OMPST_V2/Weapons/BP_Weapon.BP_Weapon_C|SetAmmoCurrent _attachedweapon (Variables|Default|GetcurrentAmmo))
      (Variables|/Game/OMPST_V2/Weapons/BP_Weapon.BP_Weapon_C|SetAmmoTotal _attachedweapon (Variables|Default|GettotalAmmo))
      (Actor|DestroyActor))))

(fn ConstructionScript
  (|CallParentFunction))

(fn -attachWeapon
  (bind _tocharacter (Variables|Default|GetToCharacter))
  (bind _returnvalue (Game|SpawnActorfromClass "/Game/OMPST_V2/Weapons/BP_Weapon_ShotGun.BP_Weapon_ShotGun_C" (Math|Transform|MakeTransform "0, 0, 0" "0, 0, 0" "1,1,1") "AlwaysSpawn" (Pawn|GetController _tocharacter) _tocharacter _tocharacter))
  (bind _output_get (LocalVariables|SetL_Weapon _returnvalue))
  (Transformation|AttachActorToActor _output_get _tocharacter "None" "SnapToTarget" "SnapToTarget" "KeepRelative" true)
  (Rendering|SetActorHiddenInGame (LocalVariables|GetL_Weapon) true)
  (Variables|/Game/OMPST_V2/Weapons/BP_Weapon.BP_Weapon_C|SetAmmoCurrent (LocalVariables|GetL_Weapon) (Variables|Default|GetcurrentAmmo))
  (Variables|/Game/OMPST_V2/Weapons/BP_Weapon.BP_Weapon_C|SetAmmoTotal (LocalVariables|GetL_Weapon) (Variables|Default|GettotalAmmo)))