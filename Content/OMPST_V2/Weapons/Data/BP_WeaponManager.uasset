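; Weapon manager for BP_MainCharacter that spawns, switches and drops AK47, shotgun and sniper rifle actors.
; SpawnWeapon attaches hidden AK47 and shotgun actors to the character; the sniper spawn is disconnected.
; Server events set CurrentWeapon, whose OnRep, on the server only, moves it to the hand socket and hides the previous one.
; Dropping non-AK47 weapons spawns an ammo-preserving pickup, expires the weapon, then a timer restores the AK47 if alive.
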(event Custom|DropWeaponServer
  (params (current :type Integer) (total :type Integer))
  ;[1 1 1] Drop weapon
  (DropWeapon|-spawnDropedWeapon current total))

(event Custom|DropWeaponEvent
  (bind _currentweapon (Variables|Default|GetCurrentWeapon))
  ;[1 1 1] Drop weapon
  (CallFunction|DropWeaponServer (Variables|/Game/OMPST_V2/Weapons/BP_Weapon.BP_Weapon_C|GetAmmoCurrent _currentweapon) (Variables|/Game/OMPST_V2/Weapons/BP_Weapon.BP_Weapon_C|GetAmmoTotal _currentweapon)))

(event Custom|SelectWeaponServer
  (params (Weapon :type BP%20Weapon%20Object%20Reference) (Type :type BP_E_Weapons%20Enum :default "NewEnumerator0"))
  ;[1 1 1] Select weapon
  (CallFunction|SelectWeapon Type))

(event EventBeginPlay
  ;[1 1 1] BeginPlay
  (bind _asbp_main_character (Utilities|Casting|CastToBP_MainCharacter (Components|GetOwner)))
  (Variables|Default|SetToCharacter _asbp_main_character))

(fn SpawnWeapon
  ;[1 1 1] Spawn weapon and attaching to character
  (CallFunction|AttachWeapon "/Game/OMPST_V2/Weapons/BP_Weapon_AK47.BP_Weapon_AK47_C")
  (CallFunction|AttachWeapon "/Game/OMPST_V2/Weapons/BP_Weapon_ShotGun.BP_Weapon_ShotGun_C"))

(fn AttachWeapon
  (params (WeaponClass :type BP%20Weapon%20Class%20Reference))
  (bind _tocharacter (Variables|Default|GetToCharacter))
  ;[1 1 1] Spawn weapon and attaching to character
  (bind _returnvalue (Game|SpawnActorfromClass WeaponClass (Math|Transform|MakeTransform "0, 0, 0" "0, 0, 0" "1,1,1") "AlwaysSpawn" (Pawn|GetController _tocharacter) _tocharacter _tocharacter))
  (bind _output_get (LocalVariables|SetL_Weapon _returnvalue))
  (switch Utilities|FlowControl|Switch|SwitchonBP_E_Weapons (Variables|/Game/OMPST_V2/Weapons/BP_Weapon.BP_Weapon_C|GetWeaponType _output_get)
    (:NewEnumerator0
      (Variables|Default|SetAK47_Weapon (LocalVariables|GetL_Weapon)))
    (:NewEnumerator1
      (Variables|Default|SetSniperRifle_Weapon (LocalVariables|GetL_Weapon)))
    (:NewEnumerator2
      (Variables|Default|SetShotGun_Weapon (LocalVariables|GetL_Weapon))))
  (Transformation|AttachActorToActor (LocalVariables|GetL_Weapon) _tocharacter "None" "SnapToTarget" "SnapToTarget" "KeepRelative" true)
  (Rendering|SetActorHiddenInGame (LocalVariables|GetL_Weapon) true)
  (return (LocalVariables|GetL_Weapon)))

(fn SelectWeapon
  (params (Type :type BP_E_Weapons%20Enum :default "NewEnumerator0"))
  (bind _ak47_weapon (Variables|Default|GetAK47_Weapon))
  (bind _sniperrifle_weapon (Variables|Default|GetSniperRifle_Weapon))
  (bind _shotgun_weapon (Variables|Default|GetShotGun_Weapon))
  (bind _returnvalue (Utilities|Select :Index Type :NewEnumerator0 _ak47_weapon :NewEnumerator1 _sniperrifle_weapon :NewEnumerator2 _shotgun_weapon))
  ;[1 1 1] Select current weapon
  (Utilities|IsValid _returnvalue
    (:Is%20Valid
      (Variables|Default|SetCurrentWeapon _returnvalue))))

(fn OnRepCurrentWeapon
  ;[1 1 1] Change current weapon
  (if (Networking|IsServer)
    (bind _currentweapon (Variables|Default|GetCurrentWeapon)
      (:then
        (Rendering|SetActorHiddenInGame _currentweapon false)
        (bind _attachedweapon (Variables|Default|GetAttachedWeapon)
          (:then
            (Transformation|AttachActorToActor _attachedweapon (Variables|Default|GetToCharacter) "None" "SnapToTarget" "SnapToTarget" "KeepRelative" true)
            (Rendering|SetActorHiddenInGame (Variables|Default|GetAttachedWeapon) true))
          (:else
            _))
        (bind _currentweapon_2 (Variables|Default|GetCurrentWeapon)
          (:then
            (Transformation|AttachComponentToComponent _currentweapon_2 (Variables|/Script/Engine.Character|GetMesh (Variables|Default|GetToCharacter)) "S_Weapon" "SnapToTarget" "SnapToTarget" "KeepRelative" true)
            (Variables|Default|SetAttachedWeapon (Variables|Default|GetCurrentWeapon)))
          (:else)))
      (:else
        (Variables|Default|SetAttachedWeapon 0)))))

(fn DropWeaponStop
  (Utilities|Time|ClearandInvalidateTimerbyHandle (Variables|Default|GetDropWeaponTimer))
  (if (> (Variables|/Game/OMPST_V2/Blueprints/Player/BP_MainCharacter.BP_MainCharacter_C|GetCurrentHP (Variables|Default|GetToCharacter)) 0.0)
    (Variables|Default|SetCurrentWeapon (Variables|Default|GetAK47_Weapon))))

(fn -spawnDropedWeapon
  (params (current :type Integer) (total :type Integer))
  (bind (_loc_x _loc_y _loc_z _rot_x _rot_y _rot_z) (Dropweapon|-spawnPosition))
  ;[1 1 1] Drop weapon
  (LocalVariables|SetL_Current current)
  (LocalVariables|SetL_Total total)
  (if (!= (Variables|Default|GetCurrentWeapon) (Variables|Default|GetAK47_Weapon))
    (if (== (Variables|Default|GetCurrentWeapon) (Variables|Default|GetShotGun_Weapon))
      (Game|SpawnActorfromClass "/Game/OMPST_V2/Blueprints/Interact/BP_PickUP_ShotGun.BP_PickUP_ShotGun_C" (Math|Transform|MakeTransform (Math|Vector|MakeVector _loc_x _loc_y _loc_z) (Math|Rotator|MakeRotator _rot_x _rot_y _rot_z) "1,1,1") "AlwaysSpawn" 0 (LocalVariables|GetL_Current) (LocalVariables|GetL_Total) 0 0)
      (else
        (Game|SpawnActorfromClass "/Game/OMPST_V2/Blueprints/Interact/BP_PickUP_Sniper.BP_PickUP_Sniper_C" (Math|Transform|MakeTransform (Math|Vector|MakeVector _loc_x _loc_y _loc_z) (Math|Rotator|MakeRotator _rot_x _rot_y _rot_z) "1,1,1") "AlwaysSpawn" 0 (LocalVariables|GetL_Current) (LocalVariables|GetL_Total) 0 0)))
    (bind _currentweapon (Variables|Default|GetCurrentWeapon)
      (:then
        (Actor|SetLifeSpan _currentweapon 0.1)
        (Default|ChangeWeaponAnimServer (Variables|Default|GetToCharacter))
        (bind _returnvalue (Utilities|Time|SetTimerbyFunctionName 0 "DropWeaponStop" 1.5))
        (Variables|Default|SetDropWeaponTimer _returnvalue))
      (:else))))

(fn -spawnPosition
  (bind _tocharacter (Variables|Default|GetToCharacter))
  (bind _fpcamera (Variables|/Game/OMPST_V2/Blueprints/Player/BP_MainCharacter.BP_MainCharacter_C|GetFPCamera _tocharacter))
  (bind _returnvalue (Transformation|GetWorldLocation _fpcamera))
  (bind _returnvalue_2 (Math|Vector|GetForwardVector _fpcamera))
  (bind _returnvalue_3 (Transformation|GetWorldRotation _fpcamera))
  (bind _returnvalue_4 (* _returnvalue_2 5e+01))
  (bind _returnvalue_5 (+ _returnvalue_4 _returnvalue))
  (return (.x _returnvalue_5) (.y _returnvalue_5) (- (.z _returnvalue_5) 4e+01) (- (.roll _returnvalue_3) 1e+01) (- (.pitch _returnvalue_3) 1e+01) (.yaw _returnvalue_3)))