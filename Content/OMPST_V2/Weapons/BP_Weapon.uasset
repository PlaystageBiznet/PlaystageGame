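; BP_Weapon is a firearm Blueprint handling firing, ammo and reloading for the player character.
; Its construction script loads stats from the DT_Weapons row named by WeaponName.
; UseWeapon spends ammo, triggers character animation, recoil and damage, then starts a fire-rate timer that re-fires held automatic weapons; an empty magazine calls WeaponReload.
; A reload timer refills the magazine from reserve ammo, with fire and reload gated by state checks.
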(event Custom|UseWeapon
  ;[1 1 1] UseWeapon
  (if (> (Variables|Default|GetAmmoCurrent) 0)
    (if (CallFunction|AbletoUseWeapon)
      (Math|Integer|DecrementInt (Variables|Default|GetAmmoCurrent)
        (:%20%20
          (Variables|Default|SetDT_Weapon (Utilities|Struct|MakeBP_S_Weapons (- (.AmmoCurrent (Utilities|Struct|BreakBP_S_Weapons (Variables|Default|GetDT_Weapon))) 1)))
          (bind _asbp_main_character (Utilities|Casting|CastToBP_MainCharacter (Game|Player|GetPlayerPawn 0)))
          (Default|FireAnimServer _asbp_main_character)
          (Default|WeaponRecoil _asbp_main_character (Variables|Default|GetWeaponRecoil))
          (Default|WeaponDamage _asbp_main_character)
          (bind _returnvalue (Utilities|Time|SetTimerbyFunctionName 0 "Stop Rate Delay" (Variables|Default|GetFireDelay)))
          (Variables|Default|SetFireRateDelay _returnvalue))))
    (else
      (CallFunction|WeaponReload))))

(event Custom|WeaponReload
  ;[1 1 1] Reloading
  (if (CallFunction|AbletoReload)
    (Variables|Default|SetReloadingInProgress true)
    (bind _asbp_main_character (Utilities|Casting|CastToBP_MainCharacter (Game|GetPlayerCharacter 0)))
    (Default|AnimReloadingServer _asbp_main_character)
    (bind _returnvalue (Utilities|Time|SetTimerbyFunctionName 0 "Reloading" (Variables|Default|GetReloadDelay)))
    (Variables|Default|SetReloadingTimer _returnvalue)))

(fn ConstructionScript
  (bind _returnvalue (Utilities|GetDataTableRow "/Game/OMPST_V2/Weapons/Data/DT_Weapons.DT_Weapons" (Variables|Default|GetWeaponName))
    (:then
      (bind _output_get (Variables|Default|SetDT_Weapon _returnvalue))
      (Variables|Default|SetAmmoCurrent (.AmmoCurrent (Utilities|Struct|BreakBP_S_Weapons _output_get)))
      (Variables|Default|SetAmmoTotal (.AmmoTotal (Utilities|Struct|BreakBP_S_Weapons _output_get)))
      (Variables|Default|SetAmmoInGun (.AmmoInGun (Utilities|Struct|BreakBP_S_Weapons _output_get)))
      (Variables|Default|SetDamageMin (.DamageMin (Utilities|Struct|BreakBP_S_Weapons _output_get)))
      (Variables|Default|SetDamageMax (.DamageMax (Utilities|Struct|BreakBP_S_Weapons _output_get)))
      (Variables|Default|SetSpread (.Spread (Utilities|Struct|BreakBP_S_Weapons _output_get)))
      (Variables|Default|SetFireDelay (.FireDelay (Utilities|Struct|BreakBP_S_Weapons _output_get)))
      (Variables|Default|SetReloadDelay (.ReloadDelay (Utilities|Struct|BreakBP_S_Weapons _output_get)))
      (Variables|Default|SetWeaponRecoil (.WeaponRecoil (Utilities|Struct|BreakBP_S_Weapons _output_get)))
      (Variables|Default|SetAbleToScope (.AbleToScope (Utilities|Struct|BreakBP_S_Weapons _output_get)))
      (Variables|Default|SetMuzzleName (.MuzzleName (Utilities|Struct|BreakBP_S_Weapons _output_get)))
      (Variables|Default|SetName (.Name (Utilities|Struct|BreakBP_S_Weapons _output_get)))
      (Variables|Default|SetAbleAutoFire (.AbleAutoFire (Utilities|Struct|BreakBP_S_Weapons _output_get)))
      (Variables|Default|SetWeaponType (.WeaponType (Utilities|Struct|BreakBP_S_Weapons _output_get)))
      (Variables|Default|SetBulletsInShot (.BulletsInShot (Utilities|Struct|BreakBP_S_Weapons _output_get)))
      (Variables|Default|SetAmmoMax (.AmmoMax (Utilities|Struct|BreakBP_S_Weapons _output_get))))))

(fn StopRateDelay
  ;[1 1 1] Stop fire rate timer
  (Utilities|Time|ClearandInvalidateTimerbyHandle (Variables|Default|GetFireRateDelay))
  (bind _asbp_main_character (Utilities|Casting|CastToBP_MainCharacter (Game|Player|GetPlayerPawn 0)))
  (if (and (Variables|Default|GetAbleAutoFire) (Variables|/Game/OMPST_V2/Blueprints/Player/BP_MainCharacter.BP_MainCharacter_C|GetFireON _asbp_main_character))
    (CallFunction|UseWeapon)))

(fn AbletoReload
  (return (Math|Boolean|ANDBoolean (> (Variables|Default|GetAmmoTotal) 0) (!= (Variables|Default|GetAmmoCurrent) (Variables|Default|GetAmmoInGun)) (not (Utilities|Time|IsValidTimerHandle (Variables|Default|GetReloadingTimer))) (not (Variables|/Game/OMPST_V2/Blueprints/Player/BP_MainCharacter.BP_MainCharacter_C|GetAiming (Variables|Default|GetWeaponOwner))))))

(fn Reloading
  (Utilities|Time|ClearandInvalidateTimerbyHandle (Variables|Default|GetReloadingTimer))
  (Variables|Default|SetNeedAmmoForReload (- (Variables|Default|GetAmmoInGun) (Variables|Default|GetAmmoCurrent)))
  (if (<= (Variables|Default|GetAmmoTotal) (Variables|Default|GetNeedAmmoForReload))
    (Variables|Default|SetAmmoCurrent (+ (Variables|Default|GetAmmoCurrent) (Variables|Default|GetAmmoTotal)))
    (Variables|Default|SetAmmoTotal 0)
    (else
      (Variables|Default|SetAmmoCurrent (Variables|Default|GetAmmoInGun))
      (Variables|Default|SetAmmoTotal (- (Variables|Default|GetAmmoTotal) (Variables|Default|GetNeedAmmoForReload)))))
  (Variables|Default|SetReloadingInProgress false))

(fn AbletoUseWeapon
  (if (Variables|Default|GetReloadingInProgress)
    (return false)
    (elif (Utilities|Time|IsValidTimerHandle (Variables|Default|GetFireRateDelay))
      (return false)
      (else
        (return true)))))